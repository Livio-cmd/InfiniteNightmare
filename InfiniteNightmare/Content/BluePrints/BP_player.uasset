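; BP_player is the player character, handling mouse look, movement, jumping, hold-Shift slow walking and pause toggling.
; Movement follows the control rotation's yaw only, and Left Shift lowers the walk speed while held.
; A camera-switch FlipFlop toggles CameraFPS, hiding the actor and showing the HUD_player widget created on BeginPlay, then reverses both on the next press.
; A second FlipFlop toggles game pause.
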(event EventBeginPlay
  ;[1 1 1] Créer un widget pour l'HUD du joueur
  (bind _returnvalue (UserInterface|CreateWidget "/Game/HUD/HUD_player.HUD_player_C"))
  (bind _output_get (Variables|Default|SetHUD%20player _returnvalue))
  (Widget|SetVisibility _output_get "Hidden")
  (UserInterface|Viewport|AddtoViewport _output_get 0))

(event Input|ActionEvents|InputActionswitchCamera
  (params (Key :type Key%20Structure :default "None"))
  ;[1 1 1] Changer de camera
  (:Pressed
    (Utilities|FlowControl|FlipFlop
      (:A
        (Rendering|SetActorHiddenInGame true)
        (Widget|SetVisibility (Variables|Default|GetHUD%20player) "Visible")
        (CallFunction|ChangerCamera))
      (:B
        (Rendering|SetActorHiddenInGame false)
        (Widget|SetVisibility (Variables|Default|GetHUD%20player) "Hidden")
        (CallFunction|ChangerCamera)))))

(event Input|ActionEvents|InputActionjump
  (params (Key :type Key%20Structure :default "None"))
  ;[1 1 1] Jump du player
  (:Pressed
    (Character|Jump))
  (:Released
    (Character|StopJumping)))

(event Input|ActionEvents|InputActionPaused
  (params (Key :type Key%20Structure :default "None"))
  ;[1 1 1] Pause
  (:Pressed
    (Utilities|FlowControl|FlipFlop
      (:A
        (Game|SetGamePaused true))
      (:B
        (Game|SetGamePaused false)))))

(event Input|AxisEvents|InputAxismoveForward
  (params (AxisValue :type Float%20%28single-precision%29))
  ;[1 1 1] Mouvements du joueur
  (Pawn|Input|AddMovementInput (Math|Vector|GetForwardVector (Math|Rotator|MakeRotator 0.0 0.0 (.Yaw (Math|Rotator|BreakRotator (Pawn|GetControlRotation :!class /Script/Engine.Pawn))))) AxisValue false))

(event Input|AxisEvents|InputAxismoveRight
  (params (AxisValue :type Float%20%28single-precision%29))
  ;[1 1 1] Mouvements du joueur
  (Pawn|Input|AddMovementInput (Math|Vector|GetRightVector (Math|Rotator|MakeRotator 0.0 0.0 (.Yaw (Math|Rotator|BreakRotator (Pawn|GetControlRotation :!class /Script/Engine.Pawn))))) AxisValue false))

(event Input|AxisEvents|InputAxisTurn
  (params (AxisValue :type Float%20%28single-precision%29))
  ;[1 1 1] Mouvements de souris
  (Pawn|Input|AddControllerYawInput AxisValue))

(event Input|AxisEvents|InputAxislookUp
  (params (AxisValue :type Float%20%28single-precision%29))
  ;[1 1 1] Mouvements de souris
  (Pawn|Input|AddControllerPitchInput AxisValue))

(event Input|KeyboardEvents|LeftShift
  (params (Key :type Key%20Structure :default "None"))
  (bind _charactermovement (Variables|Character|GetCharacterMovement))
  ;[1 1 1] Walking
  (:Pressed
    (Variables|/Script/Engine.CharacterMovementComponent|SetMaxWalkSpeed _charactermovement 1.2e+02))
  (:Released
    (Variables|/Script/Engine.CharacterMovementComponent|SetMaxWalkSpeed _charactermovement 375.0)))

(fn ConstructionScript)

(fn ChangerCamera
  (Components|Activation|ToggleActive (Variables|Default|GetcameraFPS)))